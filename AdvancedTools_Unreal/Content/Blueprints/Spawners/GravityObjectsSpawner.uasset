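; Spawner Blueprint that places gravity objects in the world when its Spawn event fires.
; The loop indexes alternately into the first two Objects classes, but its range covers one iteration, so only the first class spawns.
; Each actor lands in a random direction at SpawnRange from the world origin, owned by the spawner and stored in Spawned.
; Spawn then calls the parent BeginPlay.
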(event Custom|Spawn
  (for _index (range 0 (Variables|Default|GetObjectAmount) false 0)
    (bind _returnvalue (Game|SpawnActorfromClass (Utilities|Array|Get(acopy) (Variables|Default|GetObjects) (Math|Integer|%(Integer) _index 2)) (Math|Transform|MakeTransform (* (Math|Random|RandomUnitVector) (Variables|Default|GetSpawnRange))) "AdjustIfPossibleButAlwaysSpawn" "MultiplyWithRoot" self 0))
    (Utilities|Array|Add (Variables|Default|GetSpawned) _returnvalue))
  (|CallParentFunction))

(fn ConstructionScript
  (|CallParentFunction))