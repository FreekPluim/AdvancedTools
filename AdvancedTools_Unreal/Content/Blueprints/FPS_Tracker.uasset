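; FPS tracker Blueprint that records rounded frame-rate samples while tracking is on.
; Tick appends the rounded inverse of DeltaSeconds to the FPS array whenever the Tracking flag is set.
; CountFps toggles that flag around a next-tick delay inside a short fixed loop, leaving its Time input unused.
; The file neither clears nor reads the collected samples.
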(event Custom|CountFps
  (params (Time :type Integer))
  (for _index (range 0 Time true 1)
    (Variables|Default|SetTracking true)
    (Utilities|FlowControl|DelayUntilNextTick)
    (Variables|Default|SetTracking false)))

(event EventTick
  (params (DeltaSeconds :type Float%20%28single-precision%29))
  (if (Variables|Default|GetTracking)
    (Utilities|Array|Add (Variables|Default|GetFPS) (Math|Float|Round (/ 1.0 DeltaSeconds)))))

(fn ConstructionScript)